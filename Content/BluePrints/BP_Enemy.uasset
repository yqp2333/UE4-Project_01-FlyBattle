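; Enemy ship Blueprint that handles randomized two-tone coloring, a scale animation and a color-matched explosion effect.
; SetColor rolls body and wing colors from preset palettes, applies them through a dynamic material instance on the ship mesh, then plays the ScaleLarge timeline to animate actor scale.
; It stores both colors so SpawExplorsion can pass them as parameters to the explosion emitter it spawns at the ship's location.
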(event `self.SetColor`
  (bind _returnvalue (select `int` (`self.BodyColor`) :`0` (struct :`R` 1.0 :`G` 0.3125 :`B` 0.3125 :`A` 1.0) :`1` (struct :`R` 0.613981 :`G` 0.677083 :`B` 0.091688 :`A` 1.0) :`2` (struct :`R` 0.316772 :`G` 0.927083 :`B` 0.880926 :`A` 1.0) :`3` (struct :`R` 0.109375 :`G` 0.128134 :`B` 1.0 :`A` 1.0) :!type "LinearColor Structure"))
  (bind _returnvalue_2 (select `int` (`self.WingsColor`) :`0` (struct :`R` 0.854913 :`G` 0.949129 :`B` 1.0 :`A` 1.0) :`1` (struct :`R` 1.0 :`B` 0.026704 :`A` 1.0) :`2` (struct :`G` 0.650572 :`B` 1.0 :`A` 1.0) :`3` (struct :`R` 1.0 :`G` 0.996613 :`A` 1.0) :!type "LinearColor Structure"))
  ;[1 1 1] RandomEnemyColor
  (set `self.BodyColor` (`KismetMathLibrary.RandomIntegerInRange` 0 3))
  (set `self.WingsColor` (`KismetMathLibrary.RandomIntegerInRange` 0 3))
  (bind _returnvalue_3 (`KismetMaterialLibrary.CreateDynamicMaterialInstance` "/Game/SpaceshipBattle/Materials/M_Base_Ship.M_Base_Ship" "None"))
  (set `self.PrimaryColor` (`KismetMathLibrary.Conv_LinearColorToColor` _returnvalue))
  (`MaterialInstanceDynamic.SetVectorParameterValue` _returnvalue_3 "Color1" _returnvalue)
  (set `self.PrimaryColor2` (`KismetMathLibrary.Conv_LinearColorToColor` _returnvalue_2))
  (`MaterialInstanceDynamic.SetVectorParameterValue` _returnvalue_3 "Color2" _returnvalue_2)
  (`PrimitiveComponent.SetMaterial` (`self.ShipSM`) 0 _returnvalue_3)
  (bind (_direction _scale) (`Timeline|scaleLarge`)
    (:`Update`
      (`self.SetActorScale3D` (`KismetMathLibrary.Conv_DoubleToVector` _scale)))))

(event `self.SpawExplorsion`
  (bind _returnvalue (`GameplayStatics.SpawnEmitterAtLocation` "/Game/ParticleSystem/PS_Explorsion_Enemy.PS_Explorsion_Enemy" (`self.K2_GetActorLocation`)))
  (`FXSystemComponent.SetColorParameter` _returnvalue "Primary1" (`KismetMathLibrary.Conv_ColorToLinearColor` (`self.PrimaryColor`)))
  (`FXSystemComponent.SetColorParameter` _returnvalue "Primary2" (`KismetMathLibrary.Conv_ColorToLinearColor` (`self.PrimaryColor2`))))

(fn `UserConstructionScript`)